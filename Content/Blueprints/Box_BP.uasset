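; Box actor that acts as a simulated stick, rotating and moving while reporting its collision with a sphere.
; While simulating with nonzero RotationSpeed, Tick applies swept yaw rotation and an offset of negated Velocity, which is not scaled by delta time.
; The first sweep hit on Sphere_BP passes its normal to Physics_BP's CalculateStickRotation, with the DoOnce re-armed when simulation stops.
; Helper functions get and set the stick's relative transform.
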(event EventBeginPlay)

(event Collision|EventActorBeginOverlap
  (params (OtherActor :type Actor%20Object%20Reference)))

(event EventTick
  (params (DeltaSeconds :type Float%20%28single-precision%29))
  (if (Variables|Default|GetIsSimulating)
    (if (!= (Variables|Default|GetRotationSpeed) 0.0)
      (Transformation|AddRelativeRotation (Variables|Default|GetBox) (Math|Rotator|MakeRotator 0.0 0.0 (* DeltaSeconds (Math|Trig|RadiansToDegrees (Variables|Default|GetRotationSpeed)) -1.0)) true false)
      (bind _sweephitresult (Transformation|AddWorldOffset (Variables|Default|GetBox) (* (Variables|Default|GetVelocity) -1.0) true false))
      (if (== (Utilities|GetClass (.HitActor (Collision|BreakHitResult _sweephitresult))) "/Game/Blueprints/Sphere_BP.Sphere_BP_C")
        (Utilities|FlowControl|DoOnce false :!label _label
          (:Completed
            (bind _outactors (Actor|GetAllActorsOfClass "/Game/Blueprints/Physics_BP.Physics_BP_C"))
            (Default|CalculateStickRotation (Utilities|Array|Get(acopy) _outactors) (.Normal (Collision|BreakHitResult _sweephitresult)))))))
    (else
      (goto _label Reset))))

(fn ConstructionScript)

(fn GetStickTransform
  (bind _box (Variables|Default|GetBox))
  (return (Math|Transform|MakeTransform (Variables|/Script/Engine.SceneComponent|GetRelativeLocation _box) (Variables|/Script/Engine.SceneComponent|GetRelativeRotation _box) (Variables|/Script/Engine.SceneComponent|GetRelativeScale3D _box))))

(fn SetStickTransform
  (params (Transform :type Transform))
  (Transformation|SetRelativeTransform (Variables|Default|GetBox) Transform false false))