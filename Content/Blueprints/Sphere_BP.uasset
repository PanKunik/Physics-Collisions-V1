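; Sphere actor that moves by a velocity while simulating and reports its impact on a Box_BP.
; Tick sweeps the sphere component against the Velocity vector, scaled up and by delta time.
; The first Box_BP hit passes its normal to CalculateStickRotation on the first Physics_BP found, re-armed whenever simulation is off.
; Helper functions get and set the sphere's relative transform.
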(event EventBeginPlay)

(event EventTick
  (params (DeltaSeconds :type Float%20%28single-precision%29))
  (if (Variables|Default|GetIsSimulating)
    (if (Math|Vector|NotEqual(Vector) (Variables|Default|GetVelocity) "0, 0, 0" 0.0001)
      (bind _sweephitresult (Transformation|SetWorldLocation (Variables|Default|GetSphere) (- (Transformation|GetWorldLocation (Variables|Default|GetSphere)) (* (/ (Variables|Default|GetVelocity) 0.01) DeltaSeconds)) true false))
      (if (== (Utilities|GetClass (.HitActor (Collision|BreakHitResult _sweephitresult))) "/Game/Blueprints/Box_BP.Box_BP_C")
        (Utilities|FlowControl|DoOnce false :!label _label
          (:Completed
            (bind _outactors (Actor|GetAllActorsOfClass "/Game/Blueprints/Physics_BP.Physics_BP_C"))
            (Default|CalculateStickRotation (Utilities|Array|Get(acopy) _outactors) (.Normal (Collision|BreakHitResult _sweephitresult)))))))
    (else
      (goto _label Reset))))

(fn ConstructionScript)

(fn GetTransformSphere
  (bind _sphere (Variables|Default|GetSphere))
  (return (Math|Transform|MakeTransform (Variables|/Script/Engine.SceneComponent|GetRelativeLocation _sphere) (Variables|/Script/Engine.SceneComponent|GetRelativeRotation _sphere) (Variables|/Script/Engine.SceneComponent|GetRelativeScale3D _sphere))))

(fn SetTransformSphere
  (params (Transform :type Transform))
  (Transformation|SetRelativeTransform (Variables|Default|GetSphere) Transform false false))