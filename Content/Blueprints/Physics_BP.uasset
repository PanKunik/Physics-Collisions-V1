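; Controller for a physics simulation of a sphere colliding with a stick, with start and stop events.
; BeginPlay caches both actors' transforms and properties; starting applies masses and the widget's velocity, while stopping restores transforms and clears stick motion.
; CalculateStickRotation uses closed-form formulas, distinct for first and second hits, to set sphere velocity and stick linear and angular speed.
; A DoOnce with delayed reset debounces hits, and results display in the main widget.
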(event Custom|StartSimulation
  (bind _sphere (Variables|Default|GetSphere))
  (bind _foundwidgets (Widget|GetAllWidgetsOfClass "/Game/Widgets/UMG_MainWidget.UMG_MainWidget_C" true))
  (bind _output_get (Variables|Default|SetSphereVelocity (Math|Vector|MakeVector (Variables|/Game/Widgets/UMG_MainWidget.UMG_MainWidget_C|GetSphereVelocity (Utilities|Array|Get(acopy) _foundwidgets)) 0.0 0.0)))
  (Variables|/Game/Blueprints/Sphere_BP.Sphere_BP_C|SetVelocity _sphere _output_get)
  (Variables|/Game/Blueprints/Sphere_BP.Sphere_BP_C|SetMass _sphere (Variables|Default|GetSphereMass))
  (Variables|/Game/Blueprints/Box_BP.Box_BP_C|SetMass (Variables|Default|GetStick) (Variables|Default|GetStickMass))
  (bind _output_get_2 (Variables|Default|SetIsSimulating true))
  (bind _output_get_3 (Variables|/Game/Blueprints/Sphere_BP.Sphere_BP_C|SetIsSimulating (Variables|Default|GetSphere) _output_get_2))
  (Variables|/Game/Blueprints/Box_BP.Box_BP_C|SetIsSimulating (Variables|Default|GetStick) _output_get_3))

(event Custom|StopSimulation
  (bind _sphere (Variables|Default|GetSphere))
  (bind _stick (Variables|Default|GetStick))
  (Default|SetTransformSphere (Variables|Default|GetSphere) (Variables|Default|GetSphereTransform))
  (Default|SetStickTransform (Variables|Default|GetStick) (Variables|Default|GetStickTransform))
  (bind _output_get (Variables|Default|SetIsSimulating false))
  (bind _output_get_2 (Variables|/Game/Blueprints/Sphere_BP.Sphere_BP_C|SetIsSimulating _sphere _output_get))
  (Variables|/Game/Blueprints/Sphere_BP.Sphere_BP_C|SetVelocity _sphere (Variables|Default|GetSphereVelocity))
  (Variables|/Game/Blueprints/Box_BP.Box_BP_C|SetIsSimulating _stick _output_get_2)
  (Variables|/Game/Blueprints/Box_BP.Box_BP_C|SetRotationSpeed _stick 0.0)
  (Variables|/Game/Blueprints/Box_BP.Box_BP_C|SetVelocity _stick "0, 0, 0")
  (Variables|Default|SetCollisionCount 0))

(event Custom|CalculateStickRotation
  (params (ImpactNormal :type Vector))
  (bind _mainwidget (Variables|Default|GetMainWidget))
  (Utilities|FlowControl|DoOnce false :!label _label
    (:Completed
      (Utilities|FlowControl|Sequence
        (:then_0
          (bind _result (Math|Integer|IncrementInt (Variables|Default|GetCollisionCount))
            (:%20%20
              (switch int _result
                (:1
                  (bind _output_get (Variables|Default|SetStickRotationSpeed (Math|Vector|VectorLength (* (Variables|Default|GetSphereVelocity) (* (/ 6.0 (Variables|Default|GetStickLength)) (/ (* (Variables|Default|GetSphereMass) 2.0) (+ (* (Variables|Default|GetSphereMass) 4.0) (Variables|Default|GetStickMass))))))))
                  (Variables|/Game/Blueprints/Box_BP.Box_BP_C|SetRotationSpeed (Variables|Default|GetStick) _output_get)
                  (bind _output_get_2 (Variables|Default|SetStickVelocity (* (Variables|Default|GetSphereVelocity) (/ (* (Variables|Default|GetSphereMass) 2.0) (+ (* (Variables|Default|GetSphereMass) 4.0) (Variables|Default|GetStickMass))))))
                  (Variables|/Game/Blueprints/Box_BP.Box_BP_C|SetVelocity (Variables|Default|GetStick) _output_get_2)
                  (if (> (Variables|Default|GetStickMass) (* (Variables|Default|GetSphereMass) 4.0))
                    (bind _output_get_3 (Variables|/Game/Blueprints/Sphere_BP.Sphere_BP_C|SetVelocity (Variables|Default|GetSphere) (* (* ImpactNormal -1.0) (Math|Vector|VectorLength (* (Variables|Default|GetSphereVelocity) (/ (- (* (Variables|Default|GetSphereMass) 4.0) (Variables|Default|GetStickMass)) (+ (* (Variables|Default|GetSphereMass) 4.0) (Variables|Default|GetStickMass))))))))
                    (Variables|Default|SetSphereVelocity _output_get_3)
                    (else
                      (bind _output_get_4 (Variables|/Game/Blueprints/Sphere_BP.Sphere_BP_C|SetVelocity (Variables|Default|GetSphere) (* ImpactNormal (Math|Vector|VectorLength (* (Variables|Default|GetSphereVelocity) (/ (- (* (Variables|Default|GetSphereMass) 4.0) (Variables|Default|GetStickMass)) (+ (* (Variables|Default|GetSphereMass) 4.0) (Variables|Default|GetStickMass))))))))
                      (Variables|Default|SetSphereVelocity _output_get_4))))
                (:2
                  (bind _output_get_5 (Variables|Default|SetStickRotationSpeed (Math|Vector|VectorLength (* (Variables|Default|GetSphereVelocity) (* (/ 6.0 (Variables|Default|GetStickLength)) (/ (- (* (Variables|Default|GetSphereMass) 2.0) (Variables|Default|GetStickMass)) (+ (* (Variables|Default|GetSphereMass) 4.0) (Variables|Default|GetStickMass))))))))
                  (Variables|/Game/Blueprints/Box_BP.Box_BP_C|SetRotationSpeed (Variables|Default|GetStick) _output_get_5)
                  (bind _output_get_6 (Variables|Default|SetStickVelocity (* (Variables|Default|GetSphereVelocity) (/ (- (* (Variables|Default|GetSphereMass) 2.0) (Variables|Default|GetStickMass)) (+ (* (Variables|Default|GetSphereMass) 4.0) (Variables|Default|GetStickMass))))))
                  (Variables|/Game/Blueprints/Box_BP.Box_BP_C|SetVelocity (Variables|Default|GetStick) _output_get_6)
                  (if (> (Variables|Default|GetStickMass) (* (Variables|Default|GetSphereMass) 4.0))
                    (bind _output_get_7 (Variables|/Game/Blueprints/Sphere_BP.Sphere_BP_C|SetVelocity (Variables|Default|GetSphere) (* (* ImpactNormal -1.0) (Math|Vector|VectorLength (* (Variables|Default|GetSphereVelocity) (/ (+ (* (Variables|Default|GetSphereMass) 4.0) (Variables|Default|GetStickMass)) (- (* (Variables|Default|GetSphereMass) 4.0) (Variables|Default|GetStickMass))))))))
                    (Variables|Default|SetSphereVelocity _output_get_7)
                    (else
                      (bind _output_get_8 (Variables|/Game/Blueprints/Sphere_BP.Sphere_BP_C|SetVelocity (Variables|Default|GetSphere) (* ImpactNormal (Math|Vector|VectorLength (* (Variables|Default|GetSphereVelocity) (/ (+ (* (Variables|Default|GetSphereMass) 4.0) (Variables|Default|GetStickMass)) (- (* (Variables|Default|GetSphereMass) 4.0) (Variables|Default|GetStickMass))))))))
                      (Variables|Default|SetSphereVelocity _output_get_8)))))
              (Variables|/Game/Widgets/UMG_MainWidget.UMG_MainWidget_C|SetSphereVelAftColl _mainwidget (Utilities|String|Append (Utilities|String|ToString(Float) (Math|Vector|VectorLength (Variables|Default|GetSphereVelocity))) " m/s"))
              (Variables|/Game/Widgets/UMG_MainWidget.UMG_MainWidget_C|SetStickVelAftColl _mainwidget (Utilities|String|Append (Utilities|String|ToString(Float) (Math|Vector|VectorLength (Variables|Default|GetStickVelocity))) " m/s"))
              (Variables|/Game/Widgets/UMG_MainWidget.UMG_MainWidget_C|SetStickRotVelAftColl _mainwidget (Utilities|String|Append (Utilities|String|ToString(Float) (Variables|Default|GetStickRotationSpeed)) " rad/s")))))
        (:then_1
          (Utilities|FlowControl|Delay 0.25)
          (goto _label Reset))))))

(event EventBeginPlay
  (bind _outactors (Actor|GetAllActorsOfClass "/Game/Blueprints/Box_BP.Box_BP_C"))
  (bind _output_get (Variables|Default|SetStick (Utilities|Array|Get(acopy) _outactors)))
  (bind _transform (Default|GetStickTransform _output_get))
  (Variables|Default|SetStickTransform _transform)
  (bind _outactors_2 (Actor|GetAllActorsOfClass "/Game/Blueprints/Sphere_BP.Sphere_BP_C"))
  (bind _output_get_2 (Variables|Default|SetSphere (Utilities|Array|Get(acopy) _outactors_2)))
  (bind _transform_2 (Default|GetTransformSphere _output_get_2))
  (Variables|Default|SetSphereTransform _transform_2)
  (bind (_spheremass _spherevelocity _stickmass) (CallFunction|GetDefaultValues))
  (Variables|Default|SetSphereVelocity _spherevelocity)
  (Variables|Default|SetSphereMass _spheremass)
  (Variables|Default|SetStickMass _stickmass)
  (Variables|Default|SetStickLength (Variables|/Game/Blueprints/Box_BP.Box_BP_C|GetLength (Variables|Default|GetStick))))

(event Collision|EventActorBeginOverlap
  (params (OtherActor :type Actor%20Object%20Reference)))

(event EventTick
  (params (DeltaSeconds :type Float%20%28single-precision%29)))

(fn ConstructionScript)

(fn GetDefaultValues
  (bind _sphere (Variables|Default|GetSphere))
  (return (Variables|/Game/Blueprints/Sphere_BP.Sphere_BP_C|GetMass _sphere) (Variables|/Game/Blueprints/Sphere_BP.Sphere_BP_C|GetVelocity _sphere) (Variables|/Game/Blueprints/Box_BP.Box_BP_C|GetMass (Variables|Default|GetStick))))